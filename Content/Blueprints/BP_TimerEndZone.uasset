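; BP_TimerEndZone is a trigger zone that stops the parkour timer when BP_ParkourCharacter overlaps it.
; When IsEndOfParkour is set, it is visible and passes the timer's TrackedTime to the BP_GameMode_Parkour time event matching the current level number.
; Otherwise it is hidden in game and resets BP_Timer after stopping it, finding the timer through actor class lookups.
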(event `self.ReceiveBeginPlay`
  ;[1 1 1] SetVisibility
  (if (`self.IsEndOfParkour`)
    (`SceneComponent.SetHiddenInGame` (`self.DefaultSceneRoot`) false true)
    (else
      (`SceneComponent.SetHiddenInGame` (`self.DefaultSceneRoot`) true true))))

(event `self.ReceiveActorBeginOverlap`
  (params (OtherActor :type "Actor Object Reference"))
  ;[1 1 1] Check if player passed the line
  (cast `/Game/Blueprints/BP_ParkourCharacter` OtherActor)
  (bind _outactors (`GameplayStatics.GetAllActorsOfClass` "/Game/Blueprints/BP_Timer.BP_Timer_C"))
  (bind _output (`|GetArrayItem` _outactors))
  (set `/Game/Blueprints/BP_Timer.IsCounting` false _output)
  (if (`self.IsEndOfParkour`)
    (bind _asbp_game_mode_parkour (cast `/Game/Blueprints/BP_GameMode_Parkour` (`GameplayStatics.GetGameMode`)))
    (switch `int` (`/Game/Blueprints/BP_GameMode_Parkour.CurrentLevelNumber` _asbp_game_mode_parkour)
      (:`1`
        (bind _trackedtime (`/Game/Blueprints/BP_Timer.TrackedTime` _output))
        (`/Game/Blueprints/BP_GameMode_Parkour.Level1_TimeEvent` _asbp_game_mode_parkour _trackedtime))
      (:`2`
        (`/Game/Blueprints/BP_GameMode_Parkour.Level2_TimeEvent` _asbp_game_mode_parkour _trackedtime))
      (:`3`
        (`/Game/Blueprints/BP_GameMode_Parkour.Level3_TimeEvent` _asbp_game_mode_parkour _trackedtime))
      (:`4`
        (`/Game/Blueprints/BP_GameMode_Parkour.Level4_TimeEvent` _asbp_game_mode_parkour _trackedtime))
      (:`5`
        (`/Game/Blueprints/BP_GameMode_Parkour.Level5_TimeEvent` _asbp_game_mode_parkour _trackedtime)))
    (else
      (bind _returnvalue (`GameplayStatics.GetActorOfClass` "/Game/Blueprints/BP_Timer.BP_Timer_C"))
      (`/Game/Blueprints/BP_Timer.ResetTimer` _returnvalue))))

(fn `UserConstructionScript`)