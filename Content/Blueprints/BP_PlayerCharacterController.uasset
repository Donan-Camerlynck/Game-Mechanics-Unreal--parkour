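; Player controller for the parkour character that adds the default Enhanced Input mapping context and translates input actions into pawn actions.
; Movement is relative to control yaw, crouch and slide forward to the custom movement component, and Tick records horizontal speed.
; Dash launches along mesh axes with speed-scaled strength, a timed IsDashing flag and a cooldown.
; Reset destroys the pawn; pause shows a cached menu widget and pauses the game.
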(event `self.ReceiveBeginPlay`
  (bind _returnvalue (subsystem `EnhancedInputLocalPlayerSubsystem`))
  ;[1 1 1] Set input mapping
  (`/Engine/EditorBlueprintResources/StandardMacros.IsValid` _returnvalue
    (:`Is Valid`
      (`EnhancedInputSubsystemInterface.AddMappingContext` _returnvalue "/Game/Input/IMC_Default.IMC_Default" 0 (struct)))))

(event `self.ReceiveTick`
  (params (DeltaSeconds :type "Float (single-precision)"))
  ;[1 1 1] set velocity
  (bind _asbp_parkour_character (cast `/Game/Blueprints/BP_ParkourCharacter` (`self.K2_GetPawn`)))
  (set `self.Velocity` (`KismetMathLibrary.VSizeXY` (`CharacterMovementComponent.GetLastUpdateVelocity` (`ParkourCharacter.PlayerCharacterMovementComponent` _asbp_parkour_character)))))

(event `EnhancedInput|/Game/Input/Actions/IA_Movement`
  (params (ActionValue :type "Vector2D Structure") (ElapsedSeconds :type "Float (double-precision)") (TriggeredSeconds :type "Float (double-precision)") (InputAction :type "InputAction Object Reference" :default "/Game/Input/Actions/IA_Movement.IA_Movement"))
  (bind (_returnvalue_roll _returnvalue_pitch _returnvalue_yaw) (`KismetMathLibrary.BreakRotator` (`self.GetControlRotation`)))
  (bind (_returnvalue_roll_2 _returnvalue_pitch_2 _returnvalue_yaw_2) (`KismetMathLibrary.BreakRotator` (`self.GetControlRotation`)))
  (bind _returnvalue (`self.K2_GetPawn`))
  ;[1 1 1] input: WASD movement
  (:`Triggered`
    (`/Engine/EditorBlueprintResources/StandardMacros.IsValid` _returnvalue
      (:`Is Valid`
        (`Pawn.AddMovementInput` _returnvalue (`KismetMathLibrary.ClampVectorSize` (+ (* (`KismetMathLibrary.GetRightVector` (`KismetMathLibrary.MakeRotator` _returnvalue_roll_2 0.0 _returnvalue_yaw_2)) (* ActionValue_X -1.0)) (* (`KismetMathLibrary.GetForwardVector` (`KismetMathLibrary.MakeRotator` _returnvalue_roll 0.0 _returnvalue_yaw)) ActionValue_Y)) 0.0 1.0) 1.0 false)))))

(event `EnhancedInput|/Game/Input/Actions/IA_Look`
  (params (ActionValue :type "Vector2D Structure") (ElapsedSeconds :type "Float (double-precision)") (TriggeredSeconds :type "Float (double-precision)") (InputAction :type "InputAction Object Reference" :default "/Game/Input/Actions/IA_Look.IA_Look"))
  (bind _returnvalue (`self.K2_GetPawn`))
  ;[1 1 1] Input: mouse look
  (:`Triggered`
    (`/Engine/EditorBlueprintResources/StandardMacros.IsValid` _returnvalue
      (:`Is Valid`
        (`Pawn.AddControllerYawInput` _returnvalue ActionValue_X)
        (`Pawn.AddControllerPitchInput` _returnvalue (* ActionValue_Y -1.0))))))

(event `EnhancedInput|/Game/Input/Actions/IA_Jump`
  (params (ActionValue :type Boolean) (ElapsedSeconds :type "Float (double-precision)") (TriggeredSeconds :type "Float (double-precision)") (InputAction :type "InputAction Object Reference" :default "/Game/Input/Actions/IA_Jump.IA_Jump"))
  ;[1 1 1] Input: Jump
  (:`Triggered`
    (`/Engine/EditorBlueprintResources/StandardMacros.IsValid` (`self.K2_GetPawn`)
      (:`Is Valid`
        (`Character.Jump` (`GameplayStatics.GetPlayerCharacter` 0))))))

(event `EnhancedInput|/Game/Input/Actions/IA_Dash`
  (params (ActionValue :type Boolean) (ElapsedSeconds :type "Float (double-precision)") (TriggeredSeconds :type "Float (double-precision)") (InputAction :type "InputAction Object Reference" :default "/Game/Input/Actions/IA_Dash.IA_Dash"))
  (bind _returnvalue (`GameplayStatics.GetPlayerCharacter` 0))
  (bind _mesh (`Character.Mesh` _returnvalue))
  ;[1 1 1] Input: Dash
  (:`Triggered`
    (`/Engine/EditorBlueprintResources/StandardMacros.IsValid` (`self.K2_GetPawn`)
      (:`Is Valid`
        (if (`self.CanDash`)
          (`Character.LaunchCharacter` _returnvalue (* (`KismetMathLibrary.Normal` (+ (`SceneComponent.GetRightVector` _mesh) (* (`SceneComponent.GetUpVector` _mesh) 0.2))) (`KismetMathLibrary.MapRangeClamped` (`KismetMathLibrary.VSize` (`CharacterMovementComponent.GetLastUpdateVelocity` (`Character.CharacterMovement` _returnvalue))) 0.0 8000.0 1000.0 8000.0)) true true)
          (bind _asbp_parkour_character (cast `/Game/Blueprints/BP_ParkourCharacter` (`self.K2_GetPawn`)))
          (set `/Game/Blueprints/BP_ParkourCharacter.IsDashing` true _asbp_parkour_character)
          (set `self.CanDash` false)
          (`GameplayStatics.PlaySound2D` "/Game/Sounds/Woosh-B2-med-www_fesliyanstudios_com.Woosh-B2-med-www_fesliyanstudios_com" 1.0 1.0 0.0 null null)
          (`KismetSystemLibrary.Delay` 0.5)
          (bind _asbp_parkour_character_2 (cast `/Game/Blueprints/BP_ParkourCharacter` (`self.K2_GetPawn`)))
          (set `/Game/Blueprints/BP_ParkourCharacter.IsDashing` false _asbp_parkour_character_2)
          (`KismetSystemLibrary.Delay` 1.5)
          (set `self.CanDash` true))))))

(event `EnhancedInput|/Game/Input/Actions/IA_Reset`
  (params (ActionValue :type Boolean) (ElapsedSeconds :type "Float (double-precision)") (TriggeredSeconds :type "Float (double-precision)") (InputAction :type "InputAction Object Reference" :default "/Game/Input/Actions/IA_Reset.IA_Reset"))
  (bind _returnvalue (`self.K2_GetPawn`))
  ;[1 1 1] Reset
  (:`Triggered`
    (`/Engine/EditorBlueprintResources/StandardMacros.IsValid` _returnvalue
      (:`Is Valid`
        (`self.K2_DestroyActor` _returnvalue)))))

(event `EnhancedInput|/Game/Input/Actions/IA_Pause`
  (params (ActionValue :type Boolean) (ElapsedSeconds :type "Float (double-precision)") (TriggeredSeconds :type "Float (double-precision)") (InputAction :type "InputAction Object Reference" :default "/Game/Input/Actions/IA_Pause.IA_Pause"))
  (bind _returnvalue (`GameplayStatics.GetPlayerController` 0))
  (bind _pausemenuref (`self.PauseMenuRef`))
  ;[1 1 1] Input: Pause
  (:`Triggered`
    (`/Engine/EditorBlueprintResources/StandardMacros.IsValid` (`self.PauseMenuRef`)
      (:`Is Valid`
        _)
      (:`Is Not Valid`
        (bind _returnvalue_2 (`|CreateWidget` "/Game/Blueprints/Widgets/WB_PauseMenu.WB_PauseMenu_C"))
        (set `self.PauseMenuRef` _returnvalue_2)))
    (set `PlayerController.bShowMouseCursor` true _returnvalue)
    (`WidgetBlueprintLibrary.SetInputMode_UIOnlyEx` _returnvalue _pausemenuref)
    (`UserWidget.AddToViewport` _pausemenuref 0)
    (`GameplayStatics.SetGamePaused` true)))

(event `EnhancedInput|/Game/Input/Actions/IA_Crouch`
  (params (ActionValue :type Boolean) (ElapsedSeconds :type "Float (double-precision)") (TriggeredSeconds :type "Float (double-precision)") (InputAction :type "InputAction Object Reference" :default "/Game/Input/Actions/IA_Crouch.IA_Crouch"))
  ;[1 1 1] Input: crouch
  (:`Started`
    (bind _asbp_parkour_character (cast `/Game/Blueprints/BP_ParkourCharacter` (`self.K2_GetPawn`)))
    (`PlayerCharacterMovementComponent.CrouchPressed` (`ParkourCharacter.PlayerCharacterMovementComponent` _asbp_parkour_character))))

(event `EnhancedInput|/Game/Input/Actions/IA_Slide`
  (params (ActionValue :type Boolean) (ElapsedSeconds :type "Float (double-precision)") (TriggeredSeconds :type "Float (double-precision)") (InputAction :type "InputAction Object Reference" :default "/Game/Input/Actions/IA_Slide.IA_Slide"))
  ;[1 1 1] Input: Slide
  (:`Started`
    (bind _asbp_parkour_character (cast `/Game/Blueprints/BP_ParkourCharacter` (`self.K2_GetPawn`)))
    (`PlayerCharacterMovementComponent.SlidePressed` (`ParkourCharacter.PlayerCharacterMovementComponent` _asbp_parkour_character))))

(fn `UserConstructionScript`)