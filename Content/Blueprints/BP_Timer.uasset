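; BP_Timer is a stopwatch actor that tracks elapsed time while its IsCounting flag is set.
; Tick accumulates delta seconds into a float, converts it to a Timespan and builds an unpadded minutes:seconds:fraction string, with hundredths stored in the milliseconds field.
; The ResetTimer event stops counting and clears all tracked values; nothing in this Blueprint starts the count.
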(event `self.ReceiveTick`
  (params (DeltaSeconds :type "Float (single-precision)"))
  ;[1 1 1] Timer
  (if (`self.IsCounting`)
    (bind _output_get (set `self.TrackedTimeFloat` (+ DeltaSeconds (`self.TrackedTimeFloat`))))
    (bind _output_get_2 (set `self.TrackedTime` (`KismetMathLibrary.MakeTimespan` 0 0 0 (`KismetMathLibrary.FTrunc` _output_get) (`KismetMathLibrary.FTrunc` (mod (* _output_get 100.0) 100.0)))))
    (bind (_days _hours _minutes _seconds _milliseconds) (`KismetMathLibrary.BreakTimespan` _output_get_2))
    (set `self.TrackedTimeString` (`KismetStringLibrary.Concat_StrStr` (`KismetStringLibrary.Conv_IntToString` _minutes) ":" (`KismetStringLibrary.Conv_IntToString` _seconds) ":" (`KismetStringLibrary.Conv_IntToString` _milliseconds)))))

(event `ResetTimer`
  ;[1 1 1] reset timer
  (set `self.IsCounting` false)
  (set `self.TrackedTimeFloat` 0.0)
  (set `self.TrackedTime` (struct))
  (set `self.TrackedTimeString` ""))

(fn `UserConstructionScript`)