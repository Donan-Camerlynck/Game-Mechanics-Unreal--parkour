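; Parkour player character Blueprint that registers its respawn point and drives speed and dash visual feedback.
; On BeginPlay it stores its starting transform as the spawn transform in BP_GameMode_Parkour.
; Each tick it widens camera FOV with movement speed and shows a Niagara effect above a speed threshold.
; Tick also derives the crouch flag from Custom movement mode and shows dash particles while dashing.
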(event `self.ReceiveBeginPlay`
  ;[1 1 1] set respawn point
  (bind _asbp_game_mode_parkour (cast `/Game/Blueprints/BP_GameMode_Parkour` (`GameplayStatics.GetGameMode`)))
  (set `/Game/Blueprints/BP_GameMode_Parkour.Spawn Transform` (`self.GetTransform`) _asbp_game_mode_parkour))

(event `self.ReceiveTick`
  (params (DeltaSeconds :type "Float (single-precision)"))
  (bind _niagara (`self.Niagara`))
  (bind _returnvalue (`KismetMathLibrary.VSize` (`CharacterMovementComponent.GetLastUpdateVelocity` (`self.PlayerCharacterMovementComponent`))))
  (`|ExecutionSequence`
    (:`then_0`
      ;[1 1 1] Dynamic FOV
      (`CameraComponent.SetFieldOfView` (`self.Camera`) (`KismetMathLibrary.Lerp` 100.0 115.0 (`KismetMathLibrary.MapRangeClamped` _returnvalue 0.0 5000.0 0.0 1.0)))
      (if (> _returnvalue 1850.0)
        (`SceneComponent.SetHiddenInGame` _niagara false false)
        (else
          (`SceneComponent.SetHiddenInGame` _niagara true false))))
    (:`then_1`
      ;[1 1 1] check if crouching
      (set `self.IsCrouching` (`|EnumEquality` (`CharacterMovementComponent.MovementMode` (`self.PlayerCharacterMovementComponent`)) "MOVE_Custom")))
    (:`then_2`
      ;[1 1 1] dash particles visibility
      (if (`self.IsDashing`)
        (`SceneComponent.SetHiddenInGame` (`self.NiagaraDash`) false false)
        (else
          (`SceneComponent.SetHiddenInGame` (`self.NiagaraDash`) true false))))))

(fn `UserConstructionScript`)